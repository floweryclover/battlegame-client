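; Player controller for the main menu level that shows the menu and a nickname setup popup.
; On BeginPlay it creates both widgets, adds the popup over the menu, and sets UI-only input focused on the popup with the mouse cursor visible.
; When the popup's nickname-complete event fires, it moves focus to the main menu widget and removes the popup.
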(event `self.ReceiveBeginPlay`
  (bind _returnvalue (`|CreateWidget` "/Game/Levels/MainMenu/BP_MainMenuWidget.BP_MainMenuWidget_C"))
  (set `self.메인메뉴 위젯` _returnvalue)
  (`UserWidget.AddToViewport` _returnvalue 0)
  (bind _returnvalue_2 (`|CreateWidget` "/Game/Levels/MainMenu/BP_SetNickNamePopup.BP_SetNickNamePopup_C"))
  (bind _output_get (set `self.닉네임설정 팝업` _returnvalue_2))
  (`UserWidget.AddToViewport` _output_get 0)
  (add `/Game/Levels/MainMenu/BP_SetNickNamePopup.닉네임 설정 완료시` _output_get (delegate `닉네임 설정 완료시`))
  (`WidgetBlueprintLibrary.SetInputMode_UIOnlyEx` self _output_get)
  (set `self.bShowMouseCursor` true))

(event `닉네임 설정 완료시`
  (`WidgetBlueprintLibrary.SetInputMode_UIOnlyEx` self (`self.메인메뉴 위젯`))
  (`Widget.RemoveFromParent` (`self.닉네임설정 팝업`)))

(fn `UserConstructionScript`)