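; Battle game mode that turns game signals into entities and HUD updates for a team-scored match.
; On BeginPlay it registers itself as context, then events spawn, respawn, possess and despawn BP_Player pawns tracked in an EntityId map.
; Moves go through the MovableEntity interface, skipping the locally possessed pawn.
; Timer and score reach the player controller and HUD, nicknames fill name tags, and game state and data are rebroadcast through dispatchers.
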(event `self.ReceiveBeginPlay`
  (`BattleGameBpFunctionLibrary.SetGameModeContext` self)
  (`BattleGameCtsRpc.NotifyBattleGamePrepared`))

(event `self.OnDespawnEntity`
  (params (entityId :type Integer))
  (bind _value (`BlueprintMapLibrary.Map_Find` (`self.mEntities`) entityId))
  (if (`BlueprintMapLibrary.Map_Contains` (`self.mEntities`) entityId)
    (`/Engine/EditorBlueprintResources/StandardMacros.IsValid` _value
      (:`Is Valid`
        (`self.K2_DestroyActor` _value))
      (:`Is Not Valid`
        _))
    (`BlueprintMapLibrary.Map_Remove` (`self.mEntities`) entityId)))

(event `self.OnSpawnEntity`
  (params (entityId :type Integer) (location :type "Vector Structure (by ref)") (direction :type "Float (double-precision)"))
  (bind _returnvalue (`|SpawnActorFromClass` "/Game/Entities/Player/BP_Player.BP_Player_C" (`KismetMathLibrary.MakeTransform` location (`KismetMathLibrary.MakeRotator` 0.0 0.0 direction)) "AlwaysSpawn" "MultiplyWithRoot" null null))
  (`GameEntity.SetEntityId` (cast `GameEntity` _returnvalue :!pure true) entityId)
  (`Pawn.SpawnDefaultController` _returnvalue)
  (`BlueprintMapLibrary.Map_Add` (`self.mEntities`) entityId _returnvalue))

(event `self.OnPossessEntity`
  (params (entityId :type Integer))
  (set `self.이 플레이어가 조종 중인 폰` entityId)
  (`Controller.Possess` (`GameplayStatics.GetPlayerController` 0) (`BlueprintMapLibrary.Map_Find` (`self.mEntities`) entityId)))

(event `self.OnMoveEntity`
  (params (entityId :type Integer) (location :type "Vector Structure (by ref)") (direction :type "Float (double-precision)"))
  (bind _value (`BlueprintMapLibrary.Map_Find` (`self.mEntities`) entityId))
  (if (!= (`self.이 플레이어가 조종 중인 폰`) entityId)
    (if (`BlueprintMapLibrary.Map_Contains` (`self.mEntities`) entityId)
      (if (and (`KismetSystemLibrary.IsValid` _value) (`KismetSystemLibrary.DoesImplementInterface` _value "/Script/BattleGame.MovableEntity"))
        (`MovableEntity.OnMove` (cast `MovableEntity` _value :!pure true) location direction)))))

(event `self.OnSetTimer`
  (params (seconds :type Integer) (text :type "Text (by ref)"))
  (`/Game/Levels/Battle/BP_BattleGamePlayerController.타이머 설정` (cast `/Game/Levels/Battle/BP_BattleGamePlayerController` (`GameplayStatics.GetPlayerController` 0) :!pure true) seconds text))

(event `self.OnSignalGameState`
  (params (signal :type Integer))
  (`self.게임 상태 변경시` signal))

(event `self.OnRespawnEntity`
  (params (entityId :type Integer) (location :type "Vector Structure (by ref)") (direction :type "Float (double-precision)"))
  (`|ExecutionSequence`
    (:`then_0`
      (if (not (not (`BlueprintMapLibrary.Map_Contains` (`self.mEntities`) entityId)))
        (`/Engine/EditorBlueprintResources/StandardMacros.IsValid` (`BlueprintMapLibrary.Map_Find` (`self.mEntities`) entityId)
          (:`Is Not Valid`
            (`BlueprintMapLibrary.Map_Remove` (`self.mEntities`) entityId))))
      (bind _returnvalue (`|SpawnActorFromClass` "/Game/Entities/Player/BP_Player.BP_Player_C" (`KismetMathLibrary.MakeTransform` location (`KismetMathLibrary.MakeRotator` 0.0 0.0 direction)) "Undefined" "MultiplyWithRoot" null null))
      (`GameEntity.SetEntityId` _returnvalue entityId)
      (`BlueprintMapLibrary.Map_Add` (`self.mEntities`) entityId _returnvalue))
    (:`then_1`
      (`SceneComponent.K2_SetWorldTransform` (`Actor.RootComponent` (`BlueprintMapLibrary.Map_Find` (`self.mEntities`) entityId)) (`KismetMathLibrary.MakeTransform` location (`KismetMathLibrary.MakeRotator` 0.0 0.0 direction)) false true))))

(event `self.OnSetScore`
  (params (team :type Integer) (score :type Integer))
  (if (== team 0)
    (`/Game/Levels/Battle/BP_BattleHud.승리 점수 설정` (`/Game/Levels/Battle/BP_BattleGamePlayerController.게임 HUD` (cast `/Game/Levels/Battle/BP_BattleGamePlayerController` (`GameplayStatics.GetPlayerController` 0) :!pure true)) score)
    (elif (== (`self.내 팀 ID`) team)
      (`/Game/Levels/Battle/BP_BattleHud.플레이어 점수 설정` (`/Game/Levels/Battle/BP_BattleGamePlayerController.게임 HUD` (cast `/Game/Levels/Battle/BP_BattleGamePlayerController` (`GameplayStatics.GetPlayerController` 0) :!pure true)) true score)
      (else
        (`/Game/Levels/Battle/BP_BattleHud.플레이어 점수 설정` (`/Game/Levels/Battle/BP_BattleGamePlayerController.게임 HUD` (cast `/Game/Levels/Battle/BP_BattleGamePlayerController` (`GameplayStatics.GetPlayerController` 0) :!pure true)) false score)))))

(event `self.OnAssignTeamId`
  (params (teamId :type Integer))
  (set `self.내 팀 ID` teamId))

(event `self.OnAssignEntityNickname`
  (params (entityId :type Integer) (nickname :type "Text (by ref)"))
  (bind _mentities (`self.mEntities`))
  (bind _value (`BlueprintMapLibrary.Map_Find` _mentities entityId))
  (if (and (`BlueprintMapLibrary.Map_Contains` _mentities entityId) (`KismetSystemLibrary.IsValid` _value))
    (bind _asbp_player (cast `/Game/Entities/Player/BP_Player` _value))
    (`/Game/Levels/Battle/BP_NameTagWidget.이름표 텍스트 설정` (cast `/Game/Levels/Battle/BP_NameTagWidget` (`WidgetComponent.GetWidget` (`/Game/Entities/Player/BP_Player.NameTagWidget` _asbp_player)) :!pure true) nickname)
    (`BlueprintMapLibrary.Map_Add` (`self.엔티티 닉네임 저장`) entityId nickname)))

(event `self.OnSendGameData`
  (params (myNickname :type String) (opponentNickname :type String))
  (`self.게임 데이터 수신시` (`KismetTextLibrary.Conv_StringToText` myNickname) (`KismetTextLibrary.Conv_StringToText` opponentNickname)))

(fn `UserConstructionScript`)