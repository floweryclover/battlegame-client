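; Player controller for battle levels that manages the HUD, wait screen and result screen and takes control of the player's pawn.
; BeginPlay adds input mapping and widgets, then binds to the game mode's state-change event, which toggles the wait and result screens, input mode and cursor.
; Tick possesses the pawn whose ID the game mode stores, looked up in MEntities, whenever none is controlled.
; Timer and match-result events forward data to the widgets.
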(event `self.ReceiveTick`
  (params (DeltaSeconds :type "Float (single-precision)"))
  (bind _asbp_battle_game_mode (cast `/Game/Levels/Battle/BP_BattleGameMode` (`GameplayStatics.GetGameMode`) :!pure true))
  (bind `_이_플레이어가_조종_중인_폰` (`/Game/Levels/Battle/BP_BattleGameMode.이 플레이어가 조종 중인 폰` _asbp_battle_game_mode))
  (bind _mentities (`BattleGameMode.mEntities` _asbp_battle_game_mode))
  (bind _value (`BlueprintMapLibrary.Map_Find` _mentities `_이_플레이어가_조종_중인_폰`))
  (if (and (not (`KismetSystemLibrary.IsValid` (`self.K2_GetPawn`))) (!= `_이_플레이어가_조종_중인_폰` 0) (`BlueprintMapLibrary.Map_Contains` _mentities `_이_플레이어가_조종_중인_폰`) (`KismetSystemLibrary.IsValid` _value))
    (`self.Possess` _value)))

(event `self.ReceiveBeginPlay`
  (`|ExecutionSequence`
    (:`then_0`
      (set `self.bShowMouseCursor` false)
      (`WidgetBlueprintLibrary.SetInputMode_GameOnly` self)
      (`EnhancedInputSubsystemInterface.AddMappingContext` (subsystem `EnhancedInputLocalPlayerSubsystem`) "/Game/Entities/Player/IMC_Default.IMC_Default" 0 (struct))
      (bind _returnvalue (`|CreateWidget` "/Game/Levels/Battle/BP_BattleHud.BP_BattleHud_C"))
      (bind _output_get (set `self.게임 HUD` _returnvalue))
      (`UserWidget.AddToViewport` _output_get 0)
      (bind _returnvalue_2 (`|CreateWidget` "/Game/Levels/Battle/BP_GameWaitScreen.BP_GameWaitScreen_C"))
      (bind _output_get_2 (set `self.게임 준비 위젯` _returnvalue_2))
      (`UserWidget.AddToViewport` _output_get_2 0)
      (bind _returnvalue_3 (`|CreateWidget` "/Game/Levels/Battle/BP_GameResultScreen.BP_GameResultScreen_C"))
      (bind _output_get_3 (set `self.게임 결과 위젯` _returnvalue_3))
      (set `Widget.Visibility` "Collapsed" _output_get_3)
      (`UserWidget.AddToViewport` _output_get_3 0))
    (:`then_1`
      (add `/Game/Levels/Battle/BP_BattleGameMode.게임 상태 변경시` (cast `/Game/Levels/Battle/BP_BattleGameMode` (`GameplayStatics.GetGameMode`) :!pure true) (`|CreateDelegate` :!event `게임 상태 변경시`)))))

(event `타이머 설정`
  (params (`초` :type Integer) (`텍스트` :type Text))
  (`/Game/Levels/Battle/BP_BattleHud.타이머 설정` (`self.게임 HUD`) `초` `텍스트`))

(event `게임 상태 변경시`
  (params (`게임 상태 신호` :type Integer))
  (switch `int` `게임 상태 신호`
    (:`1`
      (set `Widget.Visibility` "Visible" (`self.게임 준비 위젯`))
      (`WidgetBlueprintLibrary.SetInputMode_UIOnlyEx` self (`self.게임 준비 위젯`))
      (set `self.bShowMouseCursor` true))
    (:`2`
      (set `Widget.Visibility` "Collapsed" (`self.게임 준비 위젯`))
      (`WidgetBlueprintLibrary.SetInputMode_GameOnly` self)
      (set `self.bShowMouseCursor` false))
    (:`3`
      (set `Widget.Visibility` "Visible" (`self.게임 결과 위젯`))
      (`WidgetBlueprintLibrary.SetInputMode_UIOnlyEx` self (`self.게임 결과 위젯`))
      (set `self.bShowMouseCursor` true))))

(event `게임 결과 수신시`
  (params (`정상적인 게임인지` :type Boolean) (`내가 이겼는지` :type Boolean) (`내 점수` :type Integer) (`상대 점수` :type Integer))
  (bind `_게임_결과_위젯` (`self.게임 결과 위젯`)
    (:`then`
      (`/Game/Levels/Battle/BP_GameResultScreen.게임 결과 수신시` `_게임_결과_위젯` `정상적인 게임인지` `내가 이겼는지` `내 점수` `상대 점수`))
    (:`else`)))

(fn `UserConstructionScript`)